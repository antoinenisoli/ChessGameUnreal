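; Board actor that builds a checkerboard of static mesh tiles at BeginPlay.
; Nested loops add mesh components on a 100-unit grid, picking white or black material from the parity of the summed indices.
; Both loops run from 1 to 0, so as written no tiles are spawned.
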(event EventBeginPlay
  (for _index (range 1 0)
    (for _index_2 (range 1 0)
      (bind _returnvalue (AddComponent|AddStaticMeshComponent false (Math|Transform|MakeTransform (Math|Vector|MakeVector (Math|Conversions|ToFloat(Integer) (* _index_2 100)) (Math|Conversions|ToFloat(Integer) (* _index 100)) 0.0))))
      (Rendering|Material|SetMaterial _returnvalue 0 (Utilities|Select :Index (Math|Integer|%(Integer) (+ _index_2 _index) 2) :Option%200 (Variables|Default|GetwhiteTile) :Option%201 (Variables|Default|GetblackTile))))))

(event Collision|EventActorBeginOverlap
  (params (OtherActor :type Actor%20Object%20Reference)))

(event EventTick
  (params (DeltaSeconds :type Float%20%28single-precision%29)))

(fn ConstructionScript)